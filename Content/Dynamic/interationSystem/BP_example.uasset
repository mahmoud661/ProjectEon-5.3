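; Example interactable actor for the interaction system that shows an input prompt and prints "Hello" when interacted with.
; When a BP_Stranger_Assassin enters the Box trigger, it shows the Key sprite, picking an Xbox icon or the F key from that character's GamePad value.
; Leaving the box hides the prompt.
; The Interacte event prints through a DoOnce that resets immediately afterwards.
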(event OnComponentBeginOverlap(Box)
  (params (OverlappedComponent :type Primitive%20Component%20Object%20Reference) (OtherActor :type Actor%20Object%20Reference) (OtherComp :type Primitive%20Component%20Object%20Reference) (OtherBodyIndex :type Integer) (bFromSweep :type Boolean) (SweepResult :type Hit%20Result%20Structure%20%28by%20ref%29))
  (bind _key (Variables|Default|GetKey))
  (bind _asbp_stranger_assassin (Utilities|Casting|CastToBP_Stranger_Assassin OtherActor))
  (if (== (Variables|/Game/Dynamic/BluePrints/Characters/Assassin/BP_Stranger_Assassin.BP_Stranger_Assassin_C|GetGamePad _asbp_stranger_assassin) "Xbox")
    (Rendering|Components|Sprite|SetSprite _key "/Game/Dynamic/interationSystem/Keys/XGamepad/T_X_Y_White_Light_Sprite.T_X_Y_White_Light_Sprite")
    (else
      (Rendering|Components|Sprite|SetSprite _key "/Game/Dynamic/interationSystem/Keys/Keyboard_Mouse/FKey.FKey")))
  (Rendering|SetVisibility _key true false))

(event OnComponentEndOverlap(Box)
  (params (OverlappedComponent :type Primitive%20Component%20Object%20Reference) (OtherActor :type Actor%20Object%20Reference) (OtherComp :type Primitive%20Component%20Object%20Reference) (OtherBodyIndex :type Integer))
  (Rendering|SetVisibility (Variables|Default|GetKey) false false))

(event EventBeginPlay)

(event Collision|EventActorBeginOverlap
  (params (OtherActor :type Actor%20Object%20Reference)))

(event EventTick
  (params (DeltaSeconds :type Float%20%28single-precision%29)))

(event EventInteracte
  (Utilities|FlowControl|DoOnce false :!label _label
    (:Completed
      (Development|PrintString "Hello")
      (goto _label Reset))))

(fn ConstructionScript)
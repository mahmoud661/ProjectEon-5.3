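; Ability pickup actor that unlocks its configured ability for the player when interacted with.
; The Interacte event adds the ability to the player's unlocked list and sets slice attack and ghost progress to a fixed value.
; It optionally starts a message on a linked instruction actor, then spawns a pickup effect at its location and destroys itself.
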(event EventBeginPlay
  (|CallParentFunction))

(event EventTick
  (params (DeltaSeconds :type Float%20%28single-precision%29))
  (|CallParentFunction DeltaSeconds))

(event EventInteracte
  (bind _player (Variables|Default|GetPlayer))
  (Utilities|Array|Add (Variables|/Game/Dynamic/BluePrints/Characters/Assassin/BP_Stranger_Assassin.BP_Stranger_Assassin_C|GetUnlockedAblilities _player) (Variables|Default|GetAbility))
  (Variables|/Game/Dynamic/BluePrints/Characters/Assassin/BP_Stranger_Assassin.BP_Stranger_Assassin_C|SetSliceAttackProgress _player 5.0)
  (Variables|/Game/Dynamic/BluePrints/Characters/Assassin/BP_Stranger_Assassin.BP_Stranger_Assassin_C|SetGhostProgress _player 5.0)
  (if (Variables|Default|Getinstraction)
    (Class|BPIDestroyINstraction|BeginInstraction(Message) (Variables|Default|GetinstractionActor)))
  (Niagara|SpawnSystematLocation "/Game/Dynamic/Items/NS_AbilityTook.NS_AbilityTook" (Transformation|GetActorLocation))
  (Actor|DestroyActor))

(fn ConstructionScript
  (|CallParentFunction))
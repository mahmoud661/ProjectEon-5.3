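; BP_SliceAttack is an ability pickup item that unlocks an ability, by its name the slice attack, for the player.
; On its Interacte event it adds its Ability value to the player's unlocked abilities and sets the slice attack progress to a fixed value.
; It then spawns the NS_AbilityTook effect at its location and destroys itself.
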(event EventBeginPlay
  (|CallParentFunction) ; This node is disabled and will not be called.\nDrag off pins to build functionality.
)

(event Collision|EventActorBeginOverlap
  (params (OtherActor :type Actor%20Object%20Reference))
  (|CallParentFunction OtherActor) ; This node is disabled and will not be called.\nDrag off pins to build functionality.
)

(event EventTick
  (params (DeltaSeconds :type Float%20%28single-precision%29))
  (|CallParentFunction DeltaSeconds) ; This node is disabled and will not be called.\nDrag off pins to build functionality.
)

(event EventInteracte
  (bind _player (Variables|Default|GetPlayer))
  (Utilities|Array|Add (Variables|/Game/Dynamic/BluePrints/Characters/Assassin/BP_Stranger_Assassin.BP_Stranger_Assassin_C|GetUnlockedAblilities _player) (Variables|Default|GetAbility))
  (Variables|/Game/Dynamic/BluePrints/Characters/Assassin/BP_Stranger_Assassin.BP_Stranger_Assassin_C|SetSliceAttackProgress _player 5)
  (Niagara|SpawnSystematLocation "/Game/Dynamic/Items/NS_AbilityTook.NS_AbilityTook" (Transformation|GetActorLocation))
  (Actor|DestroyActor))

(fn ConstructionScript
  (|CallParentFunction))
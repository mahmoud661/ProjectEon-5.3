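; BP_EmberStone is an interactable key pickup, the Ember Stone, that the player collects.
; On interaction it optionally triggers an instruction message on a linked actor and spawns the NS_EmberTook Niagara effect at its pickup effect component.
; It then sets the EmberStone flag on the player's BP_Stranger_Assassin, fires TeleportPlayerEvent on GM_main and destroys itself.
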(event EventBeginPlay
  (|CallParentFunction))

(event EventTick
  (params (DeltaSeconds :type Float%20%28single-precision%29))
  (|CallParentFunction DeltaSeconds))

(event EventInteracte
  (if (Variables|Default|Getinstraction)
    (Class|BPIDestroyINstraction|BeginInstraction(Message) (Variables|Default|GetinstractionActor)))
  (Niagara|SpawnSystematLocation "/Game/Dynamic/Items/NS/NS_EmberTook.NS_EmberTook" (Transformation|GetWorldLocation (Variables|Default|GetNS_PickUpItem)))
  (bind _asbp_stranger_assassin (Utilities|Casting|CastToBP_Stranger_Assassin (Game|Player|GetPlayerPawn 0)))
  (Variables|/Game/Dynamic/BluePrints/Characters/Assassin/BP_Stranger_Assassin.BP_Stranger_Assassin_C|SetEmberStone _asbp_stranger_assassin true)
  (bind _asgm_main (Utilities|Casting|CastToGM_main (Game|GetGameMode)))
  (Default|TeleportPlayerEvent _asgm_main)
  (Actor|DestroyActor))

(fn ConstructionScript
  (|CallParentFunction))
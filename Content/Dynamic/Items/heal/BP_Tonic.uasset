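; BP_Tonic is an item pickup that grants the player an extra tonic when interacted with.
; Its Interacte event raises both the player's maximum and current tonic counts by one, then optionally starts an instruction message through InstractionActor.
; It then spawns the NS_ItemTook effect at its location and destroys itself.
; BeginPlay, Tick and construction only call the parent class.
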(event EventBeginPlay
  (|CallParentFunction))

(event EventTick
  (params (DeltaSeconds :type Float%20%28single-precision%29))
  (|CallParentFunction DeltaSeconds))

(event EventInteracte
  (bind _player (Variables|Default|GetPlayer))
  (Variables|/Game/Dynamic/BluePrints/Characters/Assassin/BP_Stranger_Assassin.BP_Stranger_Assassin_C|SetMaxTonics _player (+ (Variables|/Game/Dynamic/BluePrints/Characters/Assassin/BP_Stranger_Assassin.BP_Stranger_Assassin_C|GetMaxTonics _player) 1))
  (Variables|/Game/Dynamic/BluePrints/Characters/Assassin/BP_Stranger_Assassin.BP_Stranger_Assassin_C|SetTonics _player (+ (Variables|/Game/Dynamic/BluePrints/Characters/Assassin/BP_Stranger_Assassin.BP_Stranger_Assassin_C|GetTonics _player) 1))
  (if (Variables|Default|Getinstraction)
    (Class|BPIDestroyINstraction|BeginInstraction(Message) (Variables|Default|GetinstractionActor)))
  (Niagara|SpawnSystematLocation "/Game/Dynamic/Items/NS_ItemTook.NS_ItemTook" (Transformation|GetActorLocation))
  (Actor|DestroyActor))

(fn ConstructionScript
  (|CallParentFunction))
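; BP_Stranger is a combat character that deals and takes damage through a toggleable hitbox, which starts disabled.
; Overlapping another BP_Stranger passes Attack to its ReciveAttack, which lowers Health and clears animation overrides.
; Survivors jump to a hit animation node and set IsHit, with a short timer likely clearing it.
; At zero health it disables capsule collision, jumps to a death node and starts a timer, presumably for destruction.
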(event OnComponentBeginOverlap(HitBox)
  (params (OverlappedComponent :type Primitive%20Component%20Object%20Reference) (OtherActor :type Actor%20Object%20Reference) (OtherComp :type Primitive%20Component%20Object%20Reference) (OtherBodyIndex :type Integer) (bFromSweep :type Boolean) (SweepResult :type Hit%20Result%20Structure%20%28by%20ref%29))
  (bind _asbp_stranger (Utilities|Casting|CastToBP_Stranger OtherActor))
  (if (!= _asbp_stranger self)
    (CallFunction|ReciveAttack _asbp_stranger (Variables|Default|GetAttack))))

(event EventBeginPlay
  (CallFunction|SetHitBox false))

(event Collision|EventActorBeginOverlap
  (params (OtherActor :type Actor%20Object%20Reference)))

(event EventTick
  (params (DeltaSeconds :type Float%20%28single-precision%29)))

(fn ConstructionScript)

(fn ReciveAttack
  (params (Attack :type Float%20%28double-precision%29))
  (bind _output_get (Variables|Default|Sethealth (- (Variables|Default|Gethealth) Attack)))
  (Class|PaperZDAnimInstance|StopAllAnimationOverrides (Class|PaperZDCharacter|GetAnimInstance))
  (if (<= _output_get 0.0)
    (Collision|SetCollisionEnabled (Variables|Default|GetCapsuleComponent) "NoCollision")
    (Class|PaperZDAnimInstance|JumptoNode (Class|PaperZDCharacter|GetAnimInstance) "DeathJump" "None")
    (Utilities|Time|SetTimerbyEvent (EventDispatchers|CreateEvent :!event DestroyActor) 1.0)
    (else
      (Class|PaperZDAnimInstance|JumptoNode (Class|PaperZDCharacter|GetAnimInstance) "HitJump" "None")
      (Variables|Default|SetisHit true)
      (Utilities|Time|SetTimerbyEvent (EventDispatchers|CreateEvent :!event ClearHit) 0.5))))

(fn ClearHit
  (Variables|Default|SetisHit false))

(fn DestroyActor
  (Actor|DestroyActor))

(fn SetHitBox
  (params (Set%20Active :type Boolean))
  (if Set%20Active
    (Collision|SetCollisionEnabled (Variables|Default|GethitBox) "QueryOnly")
    (else
      (Collision|SetCollisionEnabled (Variables|Default|GethitBox) "NoCollision"))))
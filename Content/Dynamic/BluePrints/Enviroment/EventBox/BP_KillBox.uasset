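; BP_KillBox is a trigger volume that kills BP_Stranger1 characters on contact and can move the spawn location.
; On begin play it caches the GM_main game mode.
; Any actor overlapping the box first sets the game mode's SpawnLocation to the optional SpawnTarget's position, before any type check.
; An overlapping BP_Stranger1 then receives an attack equal to its current Health, with the box as attacker.
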(event OnComponentBeginOverlap(Box)
  (params (OverlappedComponent :type Primitive%20Component%20Object%20Reference) (OtherActor :type Actor%20Object%20Reference) (OtherComp :type Primitive%20Component%20Object%20Reference) (OtherBodyIndex :type Integer) (bFromSweep :type Boolean) (SweepResult :type Hit%20Result%20Structure%20%28by%20ref%29))
  (bind _spawntarget (Variables|Default|GetSpawnTarget))
  (Utilities|FlowControl|Sequence
    (:then_0
      (if (!= _spawntarget 0)
        (Variables|/Game/Dynamic/BluePrints/GameMode/GM_main.GM_main_C|SetSpawnLocation (Variables|Default|GetAs%20GM%20Main) (Transformation|GetActorLocation _spawntarget))))
    (:then_1
      (bind _asbp_stranger_1 (Utilities|Casting|CastToBP_Stranger1 OtherActor))
      (Default|ReciveAttack _asbp_stranger_1 (Variables|/Game/Dynamic/BluePrints/BP_Stranger1.BP_Stranger1_C|Gethealth _asbp_stranger_1) self))))

(event EventBeginPlay
  (bind _asgm_main (Utilities|Casting|CastToGM_main (Game|GetGameMode)))
  (Variables|Default|SetAs%20GM%20Main _asgm_main))

(event Collision|EventActorBeginOverlap
  (params (OtherActor :type Actor%20Object%20Reference)))

(event EventTick
  (params (DeltaSeconds :type Float%20%28single-precision%29)))

(fn ConstructionScript)
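; Trigger box actor that sends the BP_Stranger_Assassin player back to a SpawnTarget with a death-camera transition.
; Any overlap first copies the target's location into GM_main's SpawnLocation, if a target is set.
; For the assassin, it calls the death camera, waits briefly, then teleports it with zeroed rotation.
; It then calls the camera start binding and snaps the SpringArm back onto the root component.
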(event OnComponentBeginOverlap(Box)
  (params (OverlappedComponent :type Primitive%20Component%20Object%20Reference) (OtherActor :type Actor%20Object%20Reference) (OtherComp :type Primitive%20Component%20Object%20Reference) (OtherBodyIndex :type Integer) (bFromSweep :type Boolean) (SweepResult :type Hit%20Result%20Structure%20%28by%20ref%29))
  (bind _spawntarget (Variables|Default|GetSpawnTarget))
  (Utilities|FlowControl|Sequence
    (:then_0
      (if (!= _spawntarget 0)
        (Variables|/Game/Dynamic/BluePrints/GameMode/GM_main.GM_main_C|SetSpawnLocation (Variables|Default|GetAs%20GM%20Main) (Transformation|GetActorLocation _spawntarget))))
    (:then_1
      (bind _asbp_stranger_assassin (Utilities|Casting|CastToBP_Stranger_Assassin OtherActor))
      (Default|CallSetCameraDeath _asbp_stranger_assassin)
      (Utilities|FlowControl|Delay 2.0)
      (Transformation|Teleport _asbp_stranger_assassin (Transformation|GetActorLocation (Variables|Default|GetSpawnTarget)) "0, 0, 0")
      (Default|CallBindEventtoStartCamera _asbp_stranger_assassin)
      (Transformation|AttachComponentToComponent (Variables|/Game/Dynamic/BluePrints/Characters/Assassin/BP_Stranger_Assassin.BP_Stranger_Assassin_C|GetSpringArm _asbp_stranger_assassin) (Variables|/Script/Engine.Actor|GetRootComponent _asbp_stranger_assassin) "None" "SnapToTarget" "KeepRelative" "KeepRelative" true))))

(event EventBeginPlay
  (bind _asgm_main (Utilities|Casting|CastToGM_main (Game|GetGameMode)))
  (Variables|Default|SetAs%20GM%20Main _asgm_main))

(event Collision|EventActorBeginOverlap
  (params (OtherActor :type Actor%20Object%20Reference)))

(event EventTick
  (params (DeltaSeconds :type Float%20%28single-precision%29)))

(fn ConstructionScript)
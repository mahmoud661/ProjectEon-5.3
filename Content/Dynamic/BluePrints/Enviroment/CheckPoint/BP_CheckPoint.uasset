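; BP_CheckPoint is an interactable checkpoint that saves the player's data.
; Box overlap caches the BP_Stranger_Assassin player and shows a key prompt matching Xbox or keyboard input, hidden on exit.
; Each interaction sends player data to the GameInstance for saving.
; The first interaction also spawns press and persistent Niagara effects at the Plant, brightens the point light, and optionally triggers an instruction message.
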(event OnComponentBeginOverlap(Box)
  (params (OverlappedComponent :type Primitive%20Component%20Object%20Reference) (OtherActor :type Actor%20Object%20Reference) (OtherComp :type Primitive%20Component%20Object%20Reference) (OtherBodyIndex :type Integer) (bFromSweep :type Boolean) (SweepResult :type Hit%20Result%20Structure%20%28by%20ref%29))
  (bind _key (Variables|Default|GetKey))
  (bind _asbp_stranger_assassin (Utilities|Casting|CastToBP_Stranger_Assassin OtherActor))
  (Variables|Default|SetPlayer _asbp_stranger_assassin)
  (if (== (Variables|/Game/Dynamic/BluePrints/Characters/Assassin/BP_Stranger_Assassin.BP_Stranger_Assassin_C|GetGamePad _asbp_stranger_assassin) "Xbox")
    (Rendering|Components|Sprite|SetSprite _key "/Game/Dynamic/interactionSystem/Keys/XGamepad/T_X_Y_White_Light_Sprite.T_X_Y_White_Light_Sprite")
    (else
      (Rendering|Components|Sprite|SetSprite _key "/Game/Dynamic/interactionSystem/Keys/Keyboard_Mouse/FKey.FKey")))
  (Rendering|SetVisibility _key true false))

(event OnComponentEndOverlap(Box)
  (params (OverlappedComponent :type Primitive%20Component%20Object%20Reference) (OtherActor :type Actor%20Object%20Reference) (OtherComp :type Primitive%20Component%20Object%20Reference) (OtherBodyIndex :type Integer))
  (Rendering|SetVisibility (Variables|Default|GetKey) false false))

(event EventInteracte
  (bind _playerdata (Default|GetPlayerData (Variables|Default|GetPlayer)))
  (Class|BPISaveGame|SavePlayerData(Message) (Game|GetGameInstance) _playerdata)
  (Utilities|FlowControl|DoOnce false
    (:Completed
      (Niagara|SpawnSystematLocation "/Game/Dynamic/BluePrints/Enviroment/CheckPoint/NS_CheckPointPress.NS_CheckPointPress" (Transformation|GetWorldLocation (Variables|Default|Getplant)))
      (Niagara|SpawnSystematLocation "/Game/Dynamic/BluePrints/Enviroment/CheckPoint/NS_CheckPointpressed.NS_CheckPointpressed" (Transformation|GetWorldLocation (Variables|Default|Getplant)) "0, 0, 0" "1.000000,1.000000,1.000000" false)
      (Rendering|Components|Light|SetIntensity (Variables|Default|GetPointLight) 1e+04)
      (if (Variables|Default|Getinstraction)
        (Class|BPIDestroyINstraction|BeginInstraction(Message) (Variables|Default|GetInstractionActor))
        (Variables|Default|Setinstraction false)))))

(fn ConstructionScript)
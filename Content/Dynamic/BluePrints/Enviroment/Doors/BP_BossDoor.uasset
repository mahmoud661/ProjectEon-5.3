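; Interactable boss door that moves the player to a spawn target and spawns the BP_BloodMaster boss.
; On interaction, it saves the target's location as the spawn location in GM_main, cached at BeginPlay.
; It then calls the assassin character's death-camera function, waits briefly, teleports the character and calls its camera-start binding.
; The boss spawns at a hard-coded world position, with no guard against repeated interaction.
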(event EventBeginPlay
  (|CallParentFunction)
  (bind _asgm_main (Utilities|Casting|CastToGM_main (Game|GetGameMode)))
  (Variables|Default|SetAs%20GM%20Main _asgm_main))

(event Collision|EventActorBeginOverlap
  (params (OtherActor :type Actor%20Object%20Reference))
  (|CallParentFunction OtherActor) ; This node is disabled and will not be called.\nDrag off pins to build functionality.
)

(event EventTick
  (params (DeltaSeconds :type Float%20%28single-precision%29))
  (|CallParentFunction DeltaSeconds) ; This node is disabled and will not be called.\nDrag off pins to build functionality.
)

(event EventInteracte
  (bind _spawntarget (Variables|Default|GetSpawnTarget))
  (Utilities|FlowControl|Sequence
    (:then_0
      (if (!= _spawntarget 0)
        (Variables|/Game/Dynamic/BluePrints/GameMode/GM_main.GM_main_C|SetSpawnLocation (Variables|Default|GetAs%20GM%20Main) (Transformation|GetActorLocation _spawntarget))))
    (:then_1
      (bind _asbp_stranger_assassin (Utilities|Casting|CastToBP_Stranger_Assassin (Game|GetPlayerCharacter 0)))
      (Default|CallSetCameraDeath _asbp_stranger_assassin)
      (Utilities|FlowControl|Delay 2.0)
      (Transformation|Teleport _asbp_stranger_assassin (Transformation|GetActorLocation (Variables|Default|GetSpawnTarget)) "0, 0, 0")
      (Default|CallBindEventtoStartCamera _asbp_stranger_assassin)
      (Game|SpawnActorfromClass "/Game/Dynamic/BluePrints/Characters/BloodMaster/BP_BloodMaster.BP_BloodMaster_C" (Math|Transform|MakeTransform "35481.000000,0.000000,-959.000000" "0, 0, 0" "1.000000,1.000000,1.000000") "Undefined" "MultiplyWithRoot" 0 0))))

(fn ConstructionScript
  (|CallParentFunction))
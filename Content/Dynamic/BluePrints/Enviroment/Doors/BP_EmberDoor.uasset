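; BP_EmberDoor is a door Blueprint whose Interacte event starts an instruction message.
; BeginPlay runs the parent logic, then casts the game mode to GM_main and stores the reference, which the shown graphs do not use.
; Interacte checks that InstractionActor is valid before calling BeginInstractionMessage on it.
; The file contains no door movement logic, and its construction script only calls the parent.
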(event EventBeginPlay
  (|CallParentFunction)
  (bind _asgm_main (Utilities|Casting|CastToGM_main (Game|GetGameMode)))
  (Variables|Default|SetAs%20GM%20Main _asgm_main))

(event Collision|EventActorBeginOverlap
  (params (OtherActor :type Actor%20Object%20Reference))
  (|CallParentFunction OtherActor) ; This node is disabled and will not be called.\nDrag off pins to build functionality.
)

(event EventTick
  (params (DeltaSeconds :type Float%20%28single-precision%29))
  (|CallParentFunction DeltaSeconds) ; This node is disabled and will not be called.\nDrag off pins to build functionality.
)

(event EventInteracte
  (Utilities|FlowControl|Sequence
    (:then_0
      (Variables|Default|GetinstractionActor
        (:then
          (Class|BPIDestroyINstraction|BeginInstraction(Message) (Variables|Default|GetinstractionActor)))
        (:else)))))

(fn ConstructionScript
  (|CallParentFunction))
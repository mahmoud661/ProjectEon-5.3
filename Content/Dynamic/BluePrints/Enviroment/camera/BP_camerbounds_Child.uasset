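; BP_camerbounds_Child is a camera bounds actor that switches the BP_Stranger_Assassin camera between following the player and holding at this actor's location.
; Each Interacte event toggles on State: in Player, it sweeps the spring arm to the actor and detaches it in world space.
; In Actor, it reattaches the arm to the player's root, snapping location and keeping relative rotation and scale.
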(event EventBeginPlay
  (|CallParentFunction) ; This node is disabled and will not be called.\nDrag off pins to build functionality.
)

(event Collision|EventActorBeginOverlap
  (params (OtherActor :type Actor%20Object%20Reference)))

(event EventTick
  (params (DeltaSeconds :type Float%20%28single-precision%29))
  (|CallParentFunction DeltaSeconds) ; This node is disabled and will not be called.\nDrag off pins to build functionality.
)

(event EventInteracte
  (switch Utilities|FlowControl|Switch|SwitchonE_CameraState (Variables|Default|GetState)
    (:NewEnumerator0
      (bind _asbp_stranger_assassin (Utilities|Casting|CastToBP_Stranger_Assassin (Variables|Default|GetPlayer)))
      (Transformation|SetWorldLocation (Variables|/Game/Dynamic/BluePrints/Characters/Assassin/BP_Stranger_Assassin.BP_Stranger_Assassin_C|GetSpringArm _asbp_stranger_assassin) (Transformation|GetActorLocation) true false)
      (Transformation|DetachFromComponent (Variables|/Game/Dynamic/BluePrints/Characters/Assassin/BP_Stranger_Assassin.BP_Stranger_Assassin_C|GetSpringArm _asbp_stranger_assassin) "KeepWorld" "KeepRelative" "KeepRelative" true)
      (Variables|Default|SetState "NewEnumerator1"))
    (:NewEnumerator1
      (bind _asbp_stranger_assassin_2 (Utilities|Casting|CastToBP_Stranger_Assassin (Variables|Default|GetPlayer)))
      (Transformation|AttachComponentToComponent (Variables|/Game/Dynamic/BluePrints/Characters/Assassin/BP_Stranger_Assassin.BP_Stranger_Assassin_C|GetSpringArm _asbp_stranger_assassin_2) (Variables|/Script/Engine.Actor|GetRootComponent _asbp_stranger_assassin_2) "None" "SnapToTarget" "KeepRelative" "KeepRelative" true)
      (Variables|Default|SetState "NewEnumerator0"))))

(fn ConstructionScript
  (|CallParentFunction))
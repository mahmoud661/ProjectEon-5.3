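; BP_camerbounds is a camera-bounds trigger volume that pins the BP_Stranger_Assassin camera while that character is inside it.
; On overlap begin, it moves the character's SpringArm to this actor's location with a sweep, then detaches it in world space.
; On overlap end, it reattaches the SpringArm to the character's root, snapping location and keeping relative rotation and scale.
; Both events print debug strings.
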(event OnComponentBeginOverlap(Trigger)
  (params (OverlappedComponent :type Primitive%20Component%20Object%20Reference) (OtherActor :type Actor%20Object%20Reference) (OtherComp :type Primitive%20Component%20Object%20Reference) (OtherBodyIndex :type Integer) (bFromSweep :type Boolean) (SweepResult :type Hit%20Result%20Structure%20%28by%20ref%29))
  (bind _asbp_stranger_assassin (Utilities|Casting|CastToBP_Stranger_Assassin OtherActor))
  (Transformation|SetWorldLocation (Variables|/Game/Dynamic/BluePrints/Characters/Assassin/BP_Stranger_Assassin.BP_Stranger_Assassin_C|GetSpringArm _asbp_stranger_assassin) (Transformation|GetActorLocation) true false)
  (Transformation|DetachFromComponent (Variables|/Game/Dynamic/BluePrints/Characters/Assassin/BP_Stranger_Assassin.BP_Stranger_Assassin_C|GetSpringArm _asbp_stranger_assassin) "KeepWorld" "KeepRelative" "KeepRelative" true)
  (Development|PrintString "in"))

(event OnComponentEndOverlap(Trigger)
  (params (OverlappedComponent :type Primitive%20Component%20Object%20Reference) (OtherActor :type Actor%20Object%20Reference) (OtherComp :type Primitive%20Component%20Object%20Reference) (OtherBodyIndex :type Integer))
  (bind _asbp_stranger_assassin (Utilities|Casting|CastToBP_Stranger_Assassin OtherActor))
  (Transformation|AttachComponentToComponent (Variables|/Game/Dynamic/BluePrints/Characters/Assassin/BP_Stranger_Assassin.BP_Stranger_Assassin_C|GetSpringArm _asbp_stranger_assassin) (Variables|/Script/Engine.Actor|GetRootComponent _asbp_stranger_assassin) "None" "SnapToTarget" "KeepRelative" "KeepRelative" true)
  (Development|PrintString "out"))

(event EventBeginPlay)

(event EventTick
  (params (DeltaSeconds :type Float%20%28single-precision%29)))

(fn ConstructionScript)
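; Main game mode that handles pausing, player respawn and a faded teleport to a fixed location.
; IA_Pause opens WB_Pause, pauses the game and switches to UI-only input.
; TeleportPlayerEvent fades to black, moves the pawn, fades back in, then clears CanEnter on every BP_BossDoor.
; RespawnPlayer spawns and possesses a default pawn at SpawnLocation; the separate TeleportPlayer function lacks delays and never fades back in.
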(event Custom|TeleportPlayer%20Event
  (CameraFades|StartCameraFade (Game|GetPlayerCameraManager 0) 0.0 1.0 3.0 "(R=0.000000,G=0.000000,B=0.000000,A=1.000000)" true true)
  (Utilities|FlowControl|Delay 3.0)
  (Transformation|Teleport (Game|Player|GetPlayerPawn 0) "33766.000000,0.000000,-2356.000000" "0, 0, 0")
  (Utilities|FlowControl|Delay 1.0)
  (CameraFades|StartCameraFade (Game|GetPlayerCameraManager 0) 1.0 0.0 3.0 "(R=0.000000,G=0.000000,B=0.000000,A=1.000000)" true true)
  (bind _outactors (Actor|GetAllActorsOfClass "/Game/Dynamic/BluePrints/Enviroment/Doors/BP_BossDoor.BP_BossDoor_C"))
  (for _array_element _outactors
    (Variables|/Game/Dynamic/BluePrints/Enviroment/Doors/BP_BossDoor.BP_BossDoor_C|SetCanEnter _array_element false)))

(event Input|EnhancedActionEvents|EnhancedInputActionIA_Pause
  (params (ActionValue :type Boolean) (ElapsedSeconds :type Float%20%28double-precision%29) (TriggeredSeconds :type Float%20%28double-precision%29) (InputAction :type Input%20Action%20Object%20Reference :default "/Game/Dynamic/Inputs/Actions/IA_Pause.IA_Pause"))
  (:Started
    (bind _returnvalue (UserInterface|CreateWidget "/Game/Dynamic/UI/PauseUI/WB_Pause.WB_Pause_C"))
    (UserInterface|Viewport|AddtoViewport _returnvalue 0)
    (Variables|/Script/Engine.PlayerController|SetbShowMouseCursor (Game|GetPlayerController 0) true)
    (Game|SetGamePaused true)
    (Input|SetInputModeUIOnly (Game|GetPlayerController 0) 0 "DoNotLock" false)))

(event EventBeginPlay
  (Input|EnableInput (Game|GetPlayerController 0)))

(event EventTick
  (params (DeltaSeconds :type Float%20%28single-precision%29)))

(fn ConstructionScript)

(fn RespawnPlayer
  (bind _returnvalue (Game|SpawnActorfromClass (Variables|Default|GetDefaultPawnClass) (Math|Transform|MakeTransform (Variables|Default|GetSpawnLocation) "0, 0, 0" "1.000000,1.000000,1.000000") "AlwaysSpawn" "MultiplyWithRoot" 0 0))
  (Pawn|Possess (Game|GetPlayerController 0) _returnvalue))

(fn TeleportPlayer
  (CameraFades|StartCameraFade (Game|GetPlayerCameraManager 0) 0.0 1.0 3.0 "(R=0.000000,G=0.000000,B=0.000000,A=1.000000)" true true)
  (Transformation|Teleport (Game|Player|GetPlayerPawn 0) "33766.000000,0.000000,-2356.000000" "0, 0, 0")
  (CameraFades|StartCameraFade (Game|GetPlayerCameraManager 0) 0.0 1.0 3.0 "(R=0.000000,G=0.000000,B=0.000000,A=1.000000)" true true))
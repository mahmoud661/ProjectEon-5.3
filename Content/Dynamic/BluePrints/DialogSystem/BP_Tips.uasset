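; BP_Tips is a one-shot trigger box that shows an on-screen tip when BP_Stranger_Assassin overlaps it.
; It picks the Xbox, PlayStation or PC key from the player's GamePad setting and formats it into the tip text.
; Existing top-level WB_Tips widgets are removed before a new one is created.
; A Fade timeline drives widget opacity and outline alpha, then removes the widget and destroys the actor.
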(event OnComponentBeginOverlap(Box)
  (params (OverlappedComponent :type Primitive%20Component%20Object%20Reference) (OtherActor :type Actor%20Object%20Reference) (OtherComp :type Primitive%20Component%20Object%20Reference) (OtherBodyIndex :type Integer) (bFromSweep :type Boolean) (SweepResult :type Hit%20Result%20Structure%20%28by%20ref%29))
  (bind _asbp_stranger_assassin (Utilities|Casting|CastToBP_Stranger_Assassin OtherActor))
  (bind _output_get (Variables|Default|SetAs%20BP%20Stranger%20Assassin _asbp_stranger_assassin))
  (CallFunction|SetController _output_get)
  (bind _foundwidgets (Widget|GetAllWidgetsOfClass "/Game/Dynamic/UI/Tips/WB_Tips.WB_Tips_C" true))
  (for _array_element _foundwidgets
    (Widget|RemovefromParent _array_element))
  (bind _returnvalue (UserInterface|CreateWidget "/Game/Dynamic/UI/Tips/WB_Tips.WB_Tips_C"))
  (bind _output_get_2 (Variables|Default|SetTipUI _returnvalue))
  (Variables|/Script/UMG.TextBlock|SetText (Variables|/Game/Dynamic/UI/Tips/WB_Tips.WB_Tips_C|GetTipText _output_get_2) (Utilities|Text|FormatText (Variables|Default|GetTipText) (Variables|Default|GetKey)))
  (UserInterface|Viewport|AddtoViewport _output_get_2 0)
  (bind _alpha (Timeline|fade PlayFromStart)
    (:Update
      (Widget|SetRenderOpacity (Variables|Default|GetTipUI) _alpha)
      (Variables|/Script/UMG.Image|SetBrush (Variables|/Game/Dynamic/UI/Tips/WB_Tips.WB_Tips_C|GetImage_61 (Variables|Default|GetTipUI)) (Utilities|Struct|MakeSlateBrush (.drawas (Variables|/Script/UMG.Image|GetBrush (Variables|/Game/Dynamic/UI/Tips/WB_Tips.WB_Tips_C|GetImage_61 (Variables|Default|GetTipUI)))) (.tiling (Variables|/Script/UMG.Image|GetBrush (Variables|/Game/Dynamic/UI/Tips/WB_Tips.WB_Tips_C|GetImage_61 (Variables|Default|GetTipUI)))) (.mirroring (Variables|/Script/UMG.Image|GetBrush (Variables|/Game/Dynamic/UI/Tips/WB_Tips.WB_Tips_C|GetImage_61 (Variables|Default|GetTipUI)))) (.imagesize (Variables|/Script/UMG.Image|GetBrush (Variables|/Game/Dynamic/UI/Tips/WB_Tips.WB_Tips_C|GetImage_61 (Variables|Default|GetTipUI)))) (.margin (Variables|/Script/UMG.Image|GetBrush (Variables|/Game/Dynamic/UI/Tips/WB_Tips.WB_Tips_C|GetImage_61 (Variables|Default|GetTipUI)))) (Utilities|Struct|MakeSlateColor "(R=0.000000,G=0.000000,B=0.000000,A=1.000000)" "UseColor_Specified") (Utilities|Struct|MakeSlateBrushOutlineSettings (.cornerradii (.outlinesettings (Variables|/Script/UMG.Image|GetBrush (Variables|/Game/Dynamic/UI/Tips/WB_Tips.WB_Tips_C|GetImage_61 (Variables|Default|GetTipUI))))) (Utilities|Struct|MakeSlateColor (Utilities|Struct|MakeLinearColor (.r (.specifiedcolor (.color (.outlinesettings (Variables|/Script/UMG.Image|GetBrush (Variables|/Game/Dynamic/UI/Tips/WB_Tips.WB_Tips_C|GetImage_61 (Variables|Default|GetTipUI))))))) (.g (.specifiedcolor (.color (.outlinesettings (Variables|/Script/UMG.Image|GetBrush (Variables|/Game/Dynamic/UI/Tips/WB_Tips.WB_Tips_C|GetImage_61 (Variables|Default|GetTipUI))))))) (.b (.specifiedcolor (.color (.outlinesettings (Variables|/Script/UMG.Image|GetBrush (Variables|/Game/Dynamic/UI/Tips/WB_Tips.WB_Tips_C|GetImage_61 (Variables|Default|GetTipUI))))))) _alpha) (.coloruserule (.color (.outlinesettings (Variables|/Script/UMG.Image|GetBrush (Variables|/Game/Dynamic/UI/Tips/WB_Tips.WB_Tips_C|GetImage_61 (Variables|Default|GetTipUI))))))) (.width (.outlinesettings (Variables|/Script/UMG.Image|GetBrush (Variables|/Game/Dynamic/UI/Tips/WB_Tips.WB_Tips_C|GetImage_61 (Variables|Default|GetTipUI))))) (.roundingtype (.outlinesettings (Variables|/Script/UMG.Image|GetBrush (Variables|/Game/Dynamic/UI/Tips/WB_Tips.WB_Tips_C|GetImage_61 (Variables|Default|GetTipUI))))) true) (.resourceobject (Variables|/Script/UMG.Image|GetBrush (Variables|/Game/Dynamic/UI/Tips/WB_Tips.WB_Tips_C|GetImage_61 (Variables|Default|GetTipUI)))))))
    (:Finished
      (Widget|RemovefromParent (Variables|Default|GetTipUI))
      (Actor|DestroyActor))))

(event EventBeginPlay)

(event Collision|EventActorBeginOverlap
  (params (OtherActor :type Actor%20Object%20Reference)))

(event EventTick
  (params (DeltaSeconds :type Float%20%28single-precision%29)))

(fn ConstructionScript)

(fn SetController
  (params (Player :type BP%20Stranger%20Assassin%20Object%20Reference))
  (if (== (Variables|/Game/Dynamic/BluePrints/Characters/Assassin/BP_Stranger_Assassin.BP_Stranger_Assassin_C|GetGamePad Player) "Xbox")
    (Variables|Default|SetKey (Variables|Default|GetXboxInput))
    (elif (== (Variables|/Game/Dynamic/BluePrints/Characters/Assassin/BP_Stranger_Assassin.BP_Stranger_Assassin_C|GetGamePad (Variables|Default|GetAs%20BP%20Stranger%20Assassin)) "Playstation")
      (Variables|Default|SetKey (Variables|Default|GetPlaystation%20Input))
      (else
        (Variables|Default|SetKey (Variables|Default|GetPC))))))
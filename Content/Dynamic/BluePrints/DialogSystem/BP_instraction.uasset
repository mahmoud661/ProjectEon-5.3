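; Instruction trigger actor that shows a paused tutorial popup when its box is overlapped or BeginInstraction is called.
; It picks a key label from the player's gamepad type (Xbox, PlayStation or PC), formats it into the text and displays a WB_Instraction widget.
; Once shown, the any-key input removes the widget, destroys the actor and unpauses the game.
; A Collisions flag can disable the box, leaving only the event trigger.
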(event OnComponentBeginOverlap(Box)
  (params (OverlappedComponent :type Primitive%20Component%20Object%20Reference) (OtherActor :type Actor%20Object%20Reference) (OtherComp :type Primitive%20Component%20Object%20Reference) (OtherBodyIndex :type Integer) (bFromSweep :type Boolean) (SweepResult :type Hit%20Result%20Structure%20%28by%20ref%29))
  (bind _asbp_stranger_assassin (Utilities|Casting|CastToBP_Stranger_Assassin (Game|Player|GetPlayerPawn 0)))
  (CallFunction|SetController _asbp_stranger_assassin)
  (bind _returnvalue (UserInterface|CreateWidget "/Game/Dynamic/UI/instraction/WB_Instraction.WB_Instraction_C"))
  (bind _output_get (Variables|Default|SetUI _returnvalue))
  (Variables|/Script/UMG.TextBlock|SetText (Variables|/Game/Dynamic/UI/instraction/WB_Instraction.WB_Instraction_C|GetInstractionText _output_get) (Utilities|Text|FormatText (Variables|Default|GetInstractionText) (Variables|Default|GetKey)))
  (Variables|/Script/UMG.TextBlock|SetText (Variables|/Game/Dynamic/UI/instraction/WB_Instraction.WB_Instraction_C|GetTitle (Variables|Default|GetUI)) (Variables|Default|GetTitle))
  (UserInterface|Viewport|AddtoViewport _output_get 0)
  (Utilities|FlowControl|Sequence
    (:then_0
      (Variables|Default|SetcanDestroy true))
    (:then_1
      (Game|SetGamePaused true))))

(event Input|EnhancedActionEvents|EnhancedInputActionIA_anyKey
  (params (ActionValue :type Boolean) (ElapsedSeconds :type Float%20%28double-precision%29) (TriggeredSeconds :type Float%20%28double-precision%29) (InputAction :type Input%20Action%20Object%20Reference :default "/Game/Dynamic/Inputs/Actions/IA_anyKey.IA_anyKey"))
  (:Started
    (if (Variables|Default|GetcanDestroy)
      (Variables|Default|GetUI
        (:then
          (Widget|RemovefromParent (Variables|Default|GetUI)))
        (:else
          _))
      (Actor|DestroyActor)
      (Game|SetGamePaused false))))

(event EventBeginPlay
  (bind _returnvalue (Game|GetPlayerController 0))
  (Input|EnableInput _returnvalue)
  (if (Variables|Default|GetCollisions)
    _
    (else
      (Collision|SetCollisionEnabled (Variables|Default|GetBox) "NoCollision")))
  (Input|AddMappingContext (PlayerController|LocalPlayerSubsystems|GetEnhancedInputLocalPlayerSubsystem _returnvalue) "/Game/Dynamic/Inputs/IMC_Stranger.IMC_Stranger" 0 "(bIgnoreAllPressedKeysUntilRelease=True,bForceImmediately=False,bNotifyUserSettings=False)"))

(event EventBeginInstraction
  (bind _asbp_stranger_assassin (Utilities|Casting|CastToBP_Stranger_Assassin (Game|Player|GetPlayerPawn 0)))
  (CallFunction|SetController _asbp_stranger_assassin)
  (bind _returnvalue (UserInterface|CreateWidget "/Game/Dynamic/UI/instraction/WB_Instraction.WB_Instraction_C"))
  (bind _output_get (Variables|Default|SetUI _returnvalue))
  (Variables|/Script/UMG.TextBlock|SetText (Variables|/Game/Dynamic/UI/instraction/WB_Instraction.WB_Instraction_C|GetInstractionText _output_get) (Utilities|Text|FormatText (Variables|Default|GetInstractionText) (Variables|Default|GetKey)))
  (Variables|/Script/UMG.TextBlock|SetText (Variables|/Game/Dynamic/UI/instraction/WB_Instraction.WB_Instraction_C|GetTitle (Variables|Default|GetUI)) (Variables|Default|GetTitle))
  (UserInterface|Viewport|AddtoViewport _output_get 0)
  (Utilities|FlowControl|Sequence
    (:then_0
      (Variables|Default|SetcanDestroy true))
    (:then_1
      (Game|SetGamePaused true))))

(event EventTick
  (params (DeltaSeconds :type Float%20%28single-precision%29)))

(fn ConstructionScript)

(fn SetController
  (params (Player :type BP%20Stranger%20Assassin%20Object%20Reference))
  (if (== (Variables|/Game/Dynamic/BluePrints/Characters/Assassin/BP_Stranger_Assassin.BP_Stranger_Assassin_C|GetGamePad Player) "Xbox")
    (Variables|Default|SetKey (Variables|Default|GetXboxInput))
    (elif (== (Variables|/Game/Dynamic/BluePrints/Characters/Assassin/BP_Stranger_Assassin.BP_Stranger_Assassin_C|GetGamePad Player) "Playstation")
      (Variables|Default|SetKey (Variables|Default|GetPlaystation%20Input))
      (else
        (Variables|Default|SetKey (Variables|Default|GetPC))))))
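; BP_Dialogue is an interactable actor that shows a sequence of dialogue lines in a UI widget.
; Entering its box stores the BP_Stranger_Assassin player and shows a key prompt sprite chosen for Xbox gamepad or keyboard.
; Each Interacte event creates the widget if needed and displays the next DialogueText entry, removing it and restarting after the last line.
; Leaving the box hides the prompt, resets the index and closes the widget.
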(event OnComponentBeginOverlap(Box)
  (params (OverlappedComponent :type Primitive%20Component%20Object%20Reference) (OtherActor :type Actor%20Object%20Reference) (OtherComp :type Primitive%20Component%20Object%20Reference) (OtherBodyIndex :type Integer) (bFromSweep :type Boolean) (SweepResult :type Hit%20Result%20Structure%20%28by%20ref%29))
  (bind _key (Variables|Default|GetKey))
  (bind _asbp_stranger_assassin (Utilities|Casting|CastToBP_Stranger_Assassin OtherActor))
  (Variables|Default|SetPlayer _asbp_stranger_assassin)
  (if (== (Variables|/Game/Dynamic/BluePrints/Characters/Assassin/BP_Stranger_Assassin.BP_Stranger_Assassin_C|GetGamePad _asbp_stranger_assassin) "Xbox")
    (Rendering|Components|Sprite|SetSprite _key "/Game/Dynamic/interactionSystem/Keys/XGamepad/T_X_Y_White_Light_Sprite.T_X_Y_White_Light_Sprite")
    (else
      (Rendering|Components|Sprite|SetSprite _key "/Game/Dynamic/interactionSystem/Keys/Keyboard_Mouse/FKey.FKey")))
  (Rendering|SetVisibility _key true false))

(event OnComponentEndOverlap(Box)
  (params (OverlappedComponent :type Primitive%20Component%20Object%20Reference) (OtherActor :type Actor%20Object%20Reference) (OtherComp :type Primitive%20Component%20Object%20Reference) (OtherBodyIndex :type Integer))
  (Rendering|SetVisibility (Variables|Default|GetKey) false false)
  (Variables|Default|SetDialogueIndex 0)
  (Variables|Default|GetDialogueUI
    (:then
      (Widget|RemovefromParent (Variables|Default|GetDialogueUI))
      (Variables|Default|SetDialogueUI 0))
    (:else)))

(event EventInteracte
  (if (< (Variables|Default|GetDialogueIndex) (Utilities|Array|Length (Variables|Default|GetDialogueText)))
    (Variables|Default|GetDialogueUI
      (:then
        _)
      (:else
        (bind _returnvalue (UserInterface|CreateWidget "/Game/Dynamic/UI/Dialog/WB_Dialog.WB_Dialog_C"))
        (bind _output_get (Variables|Default|SetDialogueUI _returnvalue))
        (UserInterface|Viewport|AddtoViewport _output_get 0)))
    (Variables|/Script/UMG.TextBlock|SetText (Variables|/Game/Dynamic/UI/Dialog/WB_Dialog.WB_Dialog_C|GetDialogueText (Variables|Default|GetDialogueUI)) (Utilities|Text|ToText(String) (Utilities|Array|Get(acopy) (Variables|Default|GetDialogueText) (Variables|Default|GetDialogueIndex))))
    (else
      (Variables|Default|SetDialogueIndex -1)
      (Variables|Default|GetDialogueUI
        (:then
          (Widget|RemovefromParent (Variables|Default|GetDialogueUI))
          (Variables|Default|SetDialogueUI 0))
        (:else
          _))))
  (Math|Integer|IncrementInt (Variables|Default|GetDialogueIndex)))

(fn ConstructionScript)
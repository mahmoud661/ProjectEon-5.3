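; BP_Stranger1 is a combat character with faction, health, attack, hit and defeat states.
; Its toggleable hitbox damages overlapping Strangers of another faction, and a line trace toward the victim places Niagara impact effects.
; ReciveAttack interrupts animations and jumps to hit or death nodes, using timers for follow-up after either state.
; Dispatchers broadcast target hits, hit-state changes, death camera and defeat, while CanAct gates actions.
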(event OnComponentBeginOverlap(HitBox)
  (params (OverlappedComponent :type Primitive%20Component%20Object%20Reference) (OtherActor :type Actor%20Object%20Reference) (OtherComp :type Primitive%20Component%20Object%20Reference) (OtherBodyIndex :type Integer) (bFromSweep :type Boolean) (SweepResult :type Hit%20Result%20Structure%20%28by%20ref%29))
  (bind _asbp_stranger_1 (Utilities|Casting|CastToBP_Stranger1 OtherActor))
  (Variables|Default|SetHitedEnemy _asbp_stranger_1)
  (if (!= (Variables|Default|Getfaction) (Variables|BP_Stranger1_C|Getfaction _asbp_stranger_1))
    (Default|CallTargetHit)
    (CallFunction|ReciveAttack (Variables|Default|GetHitedEnemy) (Variables|Default|GetAttack))))

(event Custom|TargetHitEvent
  (bind _outhit (Collision|LineTraceForObjects (Transformation|GetActorLocation) (Transformation|GetActorLocation (Variables|Default|GetHitedEnemy)) (Utilities|Array|MakeArray "ObjectTypeQuery3" "ObjectTypeQuery8" "ObjectTypeQuery9") false 0 "None"))
  (Niagara|SpawnSystematLocation "/Game/Dynamic/NS/NS_EnemyHit.NS_EnemyHit" (Math|Vector|MakeVector (.x (.location _outhit)) 2e+01 (.z (.location _outhit))))
  (Niagara|SpawnSystematLocation "/Game/Dynamic/NS/NS_CageShockerHited.NS_CageShockerHited" (Math|Vector|MakeVector (.x (.location _outhit)) (.y (.location _outhit)) (.z (.location _outhit)))))

(event EventBeginPlay
  (CallFunction|SetHitBox false (Variables|Default|GetHitBox))
  (EventDispatchers|BindEventtoTargetHit (delegate Custom|TargetHitEvent)))

(event EventTick
  (params (DeltaSeconds :type Float%20%28single-precision%29)))

(fn ConstructionScript)

(fn ReciveAttack
  (params (Attack :type Float%20%28double-precision%29))
  (if (not (Variables|Default|GetisHit))
    (bind _output_get (Variables|Default|Sethealth (- (Variables|Default|Gethealth) Attack)))
    (Class|PaperZDAnimInstance|StopAllAnimationOverrides (Class|PaperZDCharacter|GetAnimInstance))
    (if (<= _output_get 0.0)
      (Variables|Default|SetIsDefeated true)
      (CallFunction|SetHitBox false (Variables|Default|GetHitBox))
      (Collision|SetCollisionEnabled (Variables|Default|GetCapsuleComponent) "NoCollision")
      (Default|CallSetCameraDeath)
      (Class|PaperZDAnimInstance|JumptoNode (Class|PaperZDCharacter|GetAnimInstance) "DeathJump" "None")
      (Utilities|Time|SetTimerbyEvent (EventDispatchers|CreateEvent :!event DestroyActor) 2.0)
      (else
        (Variables|Default|SetIsAttacking false)
        (Variables|Default|SetisHit true)
        (Class|PaperZDAnimInstance|JumptoNode (Class|PaperZDCharacter|GetAnimInstance) "HitJump" "None")
        (Default|CallIsHitChangeState true)
        (Utilities|Time|SetTimerbyEvent (EventDispatchers|CreateEvent :!event ClearHit) 0.5)))))

(fn ClearHit
  (bind _output_get (Variables|Default|SetisHit false))
  (Default|CallIsHitChangeState _output_get))

(fn DestroyActor
  (Default|CallDefeated)
  (Actor|DestroyActor))

(fn SetHitBox
  (params (Set%20Active :type Boolean) (Box :type Box%20Component%20Object%20Reference))
  (if Set%20Active
    (Collision|SetCollisionEnabled Box "QueryOnly")
    (else
      (Collision|SetCollisionEnabled Box "NoCollision"))))

(fn CanAct
  (return (Math|Boolean|ANDBoolean (not (Variables|Default|GetisHit)) (not (Variables|Default|GetIsAttacking)) (not (Variables|Default|GetIsDefeated)))))
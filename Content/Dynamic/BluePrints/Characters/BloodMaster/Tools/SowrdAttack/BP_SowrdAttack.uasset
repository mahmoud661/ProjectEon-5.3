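; BP_SowrdAttack is a BloodMaster sword attack actor that aims at the player and damages the Stranger Assassin on contact.
; On BeginPlay it disables capsule collision and plays a timeline driving the sprite's brightness and opacity.
; While CanRotate is set, Tick interpolates pitch toward the player and snaps yaw to face either side.
; Capsule overlaps call ReciveAttack on the assassin; collision re-enabling is not handled here.
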(event OnComponentBeginOverlap(Capsule)
  (params (OverlappedComponent :type Primitive%20Component%20Object%20Reference) (OtherActor :type Actor%20Object%20Reference) (OtherComp :type Primitive%20Component%20Object%20Reference) (OtherBodyIndex :type Integer) (bFromSweep :type Boolean) (SweepResult :type Hit%20Result%20Structure%20%28by%20ref%29))
  (bind _asbp_stranger_assassin (Utilities|Casting|CastToBP_Stranger_Assassin OtherActor))
  (Default|ReciveAttack _asbp_stranger_assassin 1.0))

(event EventBeginPlay
  (Collision|SetCollisionEnabled (Variables|Default|GetCapsule) "NoCollision")
  (bind _alpha (Timeline|Timeline PlayFromStart)
    (:Update
      (Rendering|Material|SetScalarParameterValueonMaterials (Variables|Default|GetSprite) "Brightnes" _alpha)
      (Rendering|Material|SetScalarParameterValueonMaterials (Variables|Default|GetSprite) "Opacity" _alpha))))

(event Collision|EventActorBeginOverlap
  (params (OtherActor :type Actor%20Object%20Reference)))

(event EventTick
  (params (DeltaSeconds :type Float%20%28single-precision%29))
  (bind _returnvalue (Transformation|GetActorLocation))
  (bind _returnvalue_2 (Game|Player|GetPlayerPawn 0))
  (bind _returnvalue_3 (Transformation|GetActorRotation))
  (bind _returnvalue_4 (Utilities|Time|GetWorldDeltaSeconds))
  (bind _returnvalue_5 (Transformation|GetActorLocation _returnvalue_2))
  (bind _returnvalue_6 (Math|Rotator|FindLookatRotation _returnvalue _returnvalue_5))
  (bind _returnvalue_7 (Math|Interpolation|RInterpTo _returnvalue_3 _returnvalue_6 _returnvalue_4 2e+01))
  (if (Variables|Default|GetCanRotate)
    (if (> (.yaw _returnvalue_7) 0.0)
      (Transformation|SetActorRotation (Math|Rotator|MakeRotator 0.0 (.pitch _returnvalue_7) 1.8e+02))
      (else
        (Transformation|SetActorRotation (Math|Rotator|MakeRotator 0.0 (.pitch _returnvalue_7) 0.0))))))

(fn ConstructionScript)
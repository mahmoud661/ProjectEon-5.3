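; Blood Master enemy character, built on a parent class with PaperZD-style animation, that fights BP_Stranger_Assassin and damages it through HitBox2 overlaps.
; Landing shakes the camera and chains land, stationary and reset animation overrides, holding the attacking state until the chain ends and capsule collision becomes Pawn.
; ReciveAttack ignores hits while already hit, otherwise reduces health, then either enters a timed hit state or disables collision and jumps to death animation and camera.
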(event OnComponentBeginOverlap(HitBox2)
  (params (OverlappedComponent :type Primitive%20Component%20Object%20Reference) (OtherActor :type Actor%20Object%20Reference) (OtherComp :type Primitive%20Component%20Object%20Reference) (OtherBodyIndex :type Integer) (bFromSweep :type Boolean) (SweepResult :type Hit%20Result%20Structure%20%28by%20ref%29))
  (bind _asbp_stranger_assassin (Utilities|Casting|CastToBP_Stranger_Assassin OtherActor))
  (CallFunction|ReciveAttack _asbp_stranger_assassin 2.0))

(event EventBeginPlay
  (|CallParentFunction)
  (Variables|Default|SetAttackAnimation "/Game/Dynamic/BluePrints/Characters/BloodMaster/AnimSequences/MoveAttack.MoveAttack")
  (Variables|Default|Sethealth 18.0))

(event Collision|EventActorBeginOverlap
  (params (OtherActor :type Actor%20Object%20Reference))
  (|CallParentFunction OtherActor) ; This node is disabled and will not be called.\nDrag off pins to build functionality.
)

(event EventTick
  (params (DeltaSeconds :type Float%20%28single-precision%29))
  (|CallParentFunction DeltaSeconds))

(event EventOnLanded
  (params (Hit :type Hit%20Result%20Structure%20%28by%20ref%29))
  (bind _returnvalue (Class|PaperZDCharacter|GetAnimInstance))
  (Camera|PlayWorldCameraShake "/Game/Dynamic/BluePrints/Characters/BloodMaster/CS_Land.CS_Land_C" (Transformation|GetActorLocation) 0.0 1e+04 0.0)
  (|PlayAnimationOverridewithCallbacks (Class|PaperZDCharacter|GetAnimInstance) "/Game/Dynamic/BluePrints/Characters/BloodMaster/AnimSequences/Land.Land" "DefaultSlot" 1.0 0.0
    (:then
      (bind _output_get (Variables|Default|SetIsAttacking true))
      (Default|CallIsAttackingChangeState _output_get))
    (:OnCompleted
      (|PlayAnimationOverridewithCallbacks _returnvalue "/Game/Dynamic/BluePrints/Characters/BloodMaster/AnimSequences/Stationary.Stationary" "DefaultSlot" 0.7 0.0
        (:OnCompleted
          (|PlayAnimationOverridewithCallbacks _returnvalue "/Game/Dynamic/BluePrints/Characters/BloodMaster/AnimSequences/Stationary_Reset.Stationary_Reset" "DefaultSlot" 1.0 0.0
            (:OnCompleted
              (bind _output_get_2 (Variables|Default|SetIsAttacking false))
              (Default|CallIsAttackingChangeState _output_get_2)
              (Collision|SetCollisionObjectType (Variables|Default|GetCapsuleComponent) "ECC_Pawn"))))))))

(fn ConstructionScript
  (|CallParentFunction))

(fn ReciveAttack
  (params (Attack :type Float%20%28double-precision%29))
  (if (not (Variables|Default|GetisHit))
    (bind _output_get (Variables|Default|Sethealth (- (Variables|Default|Gethealth) Attack)))
    (if (<= _output_get 0.0)
      (Class|PaperZDAnimInstance|StopAllAnimationOverrides (Class|PaperZDCharacter|GetAnimInstance))
      (Variables|Default|SetIsDefeated true)
      (CallFunction|SetHitBox false (Variables|Default|GetHitBox))
      (Collision|SetCollisionEnabled (Variables|Default|GetCapsuleComponent) "NoCollision")
      (Default|CallSetCameraDeath)
      (Class|PaperZDAnimInstance|JumptoNode (Class|PaperZDCharacter|GetAnimInstance) "DeathJump" "None")
      (else
        (Variables|Default|SetIsAttacking false)
        (Variables|Default|SetisHit true)
        (Default|CallIsHitChangeState true)
        (Utilities|Time|SetTimerbyEvent (EventDispatchers|CreateEvent :!event ClearHit) 0.5)))))
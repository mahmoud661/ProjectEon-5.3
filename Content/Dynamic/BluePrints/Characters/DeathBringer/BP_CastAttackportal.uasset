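; Short-lived attack portal actor for the DeathBringer character that damages the Stranger Assassin character on overlap.
; Its collision box is switched off 0.1 seconds after BeginPlay, and any BP_Stranger_Assassin that begins overlapping it receives a ReciveAttack call.
; Tick watches the Casting flipbook and destroys the actor when playback reaches the last frame.
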(event OnComponentBeginOverlap(Box)
  (params (OverlappedComponent :type Primitive%20Component%20Object%20Reference) (OtherActor :type Actor%20Object%20Reference) (OtherComp :type Primitive%20Component%20Object%20Reference) (OtherBodyIndex :type Integer) (bFromSweep :type Boolean) (SweepResult :type Hit%20Result%20Structure%20%28by%20ref%29))
  (bind _asbp_stranger_assassin (Utilities|Casting|CastToBP_Stranger_Assassin OtherActor))
  (Default|ReciveAttack _asbp_stranger_assassin 1.0))

(event EventBeginPlay
  (Utilities|FlowControl|Delay 0.1)
  (Collision|SetCollisionEnabled (Variables|Default|GetBox) "NoCollision"))

(event Collision|EventActorBeginOverlap
  (params (OtherActor :type Actor%20Object%20Reference)))

(event EventTick
  (params (DeltaSeconds :type Float%20%28single-precision%29))
  (bind _casting (Variables|Default|GetCasting))
  (if (== (Class|PaperFlipbookComponent|GetPlaybackPositioninFrames _casting) (- (Class|PaperFlipbookComponent|GetFlipbookLengthinFrames _casting) 1))
    (Actor|DestroyActor)))

(fn ConstructionScript)
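; DeathBringer enemy character that targets the player's Stranger Assassin for casting and attacking through its AI controller.
; On BeginPlay it sets its attack animation, extending the parent's logic.
; When the assassin enters the CastAggro volume, AIC_DeathBringer receives it as both cast and attack target.
; Any overlap end on that volume clears only the cast target, without checking which actor left.
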(event OnComponentBeginOverlap(CastAggro)
  (params (OverlappedComponent :type Primitive%20Component%20Object%20Reference) (OtherActor :type Actor%20Object%20Reference) (OtherComp :type Primitive%20Component%20Object%20Reference) (OtherBodyIndex :type Integer) (bFromSweep :type Boolean) (SweepResult :type Hit%20Result%20Structure%20%28by%20ref%29))
  (bind _asbp_stranger_assassin (Utilities|Casting|CastToBP_Stranger_Assassin OtherActor))
  (bind _asaic_death_bringer (Utilities|Casting|CastToAIC_DeathBringer (AI|GetAIController self)))
  (Default|SetCastTarget _asaic_death_bringer _asbp_stranger_assassin)
  (Default|SetAttackTarget _asaic_death_bringer _asbp_stranger_assassin))

(event OnComponentEndOverlap(CastAggro)
  (params (OverlappedComponent :type Primitive%20Component%20Object%20Reference) (OtherActor :type Actor%20Object%20Reference) (OtherComp :type Primitive%20Component%20Object%20Reference) (OtherBodyIndex :type Integer))
  (bind _asaic_death_bringer (Utilities|Casting|CastToAIC_DeathBringer (AI|GetAIController self)))
  (Default|SetCastTarget _asaic_death_bringer))

(event EventBeginPlay
  (|CallParentFunction)
  (Variables|Default|SetAttackAnimation "/Game/Dynamic/BluePrints/Characters/DeathBringer/AnimSequences/Attack.Attack"))

(event Collision|EventActorBeginOverlap
  (params (OtherActor :type Actor%20Object%20Reference))
  (|CallParentFunction OtherActor) ; This node is disabled and will not be called.\nDrag off pins to build functionality.
)

(event EventTick
  (params (DeltaSeconds :type Float%20%28single-precision%29))
  (|CallParentFunction DeltaSeconds) ; This node is disabled and will not be called.\nDrag off pins to build functionality.
)

(fn ConstructionScript
  (|CallParentFunction))
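; BP_OrbMage is an orb-casting mage enemy that targets BP_Stranger_Assassin and attacks with a sweep and summoned shots.
; OrbAggro overlaps set orb and attack targets on AIC_OrbMage, and leaving clears only the orb target.
; SpawnOrb samples player location, then after a brief delay spawns BP_MageShot there with OrbBox collision disabled.
; HitBox overlaps launch the assassin, and ReciveAttack extends parent handling with a low-health heal-state check.
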(event OnComponentBeginOverlap(HitBox)
  (params (OverlappedComponent :type Primitive%20Component%20Object%20Reference) (OtherActor :type Actor%20Object%20Reference) (OtherComp :type Primitive%20Component%20Object%20Reference) (OtherBodyIndex :type Integer) (bFromSweep :type Boolean) (SweepResult :type Hit%20Result%20Structure%20%28by%20ref%29))
  (bind _asbp_stranger_assassin (Utilities|Casting|CastToBP_Stranger_Assassin OtherActor))
  (Character|LaunchCharacter _asbp_stranger_assassin (Math|Vector|MakeVector (.x (* (Math|Vector|GetForwardVector (Transformation|GetActorRotation)) "600.000000,0.000000,0.000000")) 0.0 5e+02) false false))

(event OnComponentBeginOverlap(OrbAggro)
  (params (OverlappedComponent :type Primitive%20Component%20Object%20Reference) (OtherActor :type Actor%20Object%20Reference) (OtherComp :type Primitive%20Component%20Object%20Reference) (OtherBodyIndex :type Integer) (bFromSweep :type Boolean) (SweepResult :type Hit%20Result%20Structure%20%28by%20ref%29))
  (bind _asbp_stranger_assassin (Utilities|Casting|CastToBP_Stranger_Assassin OtherActor))
  (bind _asaic_orb_mage (Utilities|Casting|CastToAIC_OrbMage (AI|GetAIController self)))
  (Default|SetOrbTarget _asaic_orb_mage _asbp_stranger_assassin)
  (Default|SetAttackTarget _asaic_orb_mage _asbp_stranger_assassin))

(event OnComponentEndOverlap(OrbAggro)
  (params (OverlappedComponent :type Primitive%20Component%20Object%20Reference) (OtherActor :type Actor%20Object%20Reference) (OtherComp :type Primitive%20Component%20Object%20Reference) (OtherBodyIndex :type Integer))
  (bind _asaic_orb_mage (Utilities|Casting|CastToAIC_OrbMage (AI|GetAIController self)))
  (Default|SetOrbTarget _asaic_orb_mage))

(event Custom|SpawnOrb
  (Variables|Default|SetTargetLocation (Transformation|GetActorLocation (Game|Player|GetPlayerPawn 0)))
  (Utilities|FlowControl|Delay 0.15)
  (bind _returnvalue (Game|SpawnActorfromClass "/Game/Dynamic/BluePrints/Characters/OrbMage/Tools/BP_MageShot.BP_MageShot_C" (Math|Transform|MakeTransform (Variables|Default|GetTargetLocation) "0, 0, 0" "1.000000,1.000000,1.000000") "Undefined" "MultiplyWithRoot" 0 0))
  (Collision|SetCollisionEnabled (Variables|/Game/Dynamic/BluePrints/Characters/OrbMage/Tools/BP_MageShot.BP_MageShot_C|GetOrbBox _returnvalue) "NoCollision"))

(event EventBeginPlay
  (|CallParentFunction)
  (Variables|Default|SetAttackAnimation "/Game/Dynamic/BluePrints/Characters/OrbMage/AnimSequences/Sweep.Sweep"))

(fn ConstructionScript
  (|CallParentFunction))

(fn ReciveAttack
  (params (Attack :type Float%20%28double-precision%29))
  (|CallParentFunction Attack)
  (bind _output_get (Variables|Default|SetShouldHeal (<= (Variables|Default|Gethealth) 1.0)))
  (Default|CallShouldHealState _output_get))
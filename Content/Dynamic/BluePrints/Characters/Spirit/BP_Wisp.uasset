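; Spirit wisp character that either follows the player or leads along a tutorial route of target actors.
; Once Start is set, Tick switches on State to run FollowPlayer or TeturialLevel, steering with movement input rather than AI navigation.
; The route advances through Destinations within a fixed arrival radius and halts at the last, while follow mode halts near the player.
; A FollowMe event adds an audio component.
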(event Custom|FollowMe
  (AddComponent|AddAudioComponent false))

(event EventTick
  (params (DeltaSeconds :type Float%20%28single-precision%29))
  (if (Variables|Default|GetStart)
    (switch Utilities|FlowControl|Switch|SwitchonEN_wispState (Variables|Default|GetState)
      (:NewEnumerator0
        (CallFunction|FollowPlayer))
      (:NewEnumerator1
        (CallFunction|TeturialLevel)))))

(fn ConstructionScript)

(fn TeturialLevel
  (bind _destinations (Variables|Default|GetDestinations))
  (if (> (Transformation|GetDistanceTo (Utilities|Array|Get(acopy) (Variables|Default|GetDestinations) (Variables|Default|Gettarget))) 1e+02)
    (Pawn|Input|AddMovementInput (Math|Vector|GetForwardVector (Math|Rotator|FindLookatRotation (Transformation|GetActorLocation) (Transformation|GetActorLocation (Utilities|Array|Get(acopy) (Variables|Default|GetDestinations) (Variables|Default|Gettarget))))) 1.0 false)
    (elif (== (Utilities|Array|Get(acopy) _destinations (Variables|Default|Gettarget)) (Utilities|Array|Get(acopy) _destinations (Utilities|Array|LastIndex _destinations)))
      (Components|Movement|StopMovementImmediately (Variables|Character|GetCharacterMovement))
      (else
        (Variables|Default|Settarget (+ (Variables|Default|Gettarget) 1))))))

(fn FollowPlayer
  (if (> (Transformation|GetDistanceTo (Game|GetPlayerCharacter 0)) 1e+02)
    (Pawn|Input|AddMovementInput (Utilities|DistancetoPlayer) 1.0 false)
    (else
      (Components|Movement|StopMovementImmediately (Variables|Character|GetCharacterMovement)))))